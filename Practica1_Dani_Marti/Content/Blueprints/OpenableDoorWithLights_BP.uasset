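; Door actor that changes its yaw rotation depending on whether four referenced lights are all switched on.
; Tick checks each light's IsLightOn into AllLightsOn, then drives the DoorAmountRotation timeline, whose update sets the door mesh's relative yaw.
; All lights on calls ReverseFromEnd and any light off calls PlayFromStart, so the timeline is restarted every frame rather than only on a change.
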(event `self.ReceiveBeginPlay`)

(event `self.ReceiveTick`
  (params (DeltaSeconds :type "Float (single-precision)"))
  (`|ExecutionSequence`
    (:`then_0`
      (if (`/Game/Blueprints/PuzzleLight_BP.isLightOn` (`self.light1`))
        (if (`/Game/Blueprints/PuzzleLight_BP.isLightOn` (`self.light2`))
          (if (`/Game/Blueprints/PuzzleLight_BP.isLightOn` (`self.light3`))
            (if (`/Game/Blueprints/PuzzleLight_BP.isLightOn` (`self.light4`))
              (set `self.allLightsOn` true)
              (else
                (set `self.allLightsOn` false :!label _label)))
            (else
              (goto _label)))
          (else
            (goto _label)))
        (else
          (goto _label))))
    (:`then_1`
      (if (`self.allLightsOn`)
        (bind (_direction _doorrotationamount) (`Timeline|DoorAmountRotation` :!via `ReverseFromEnd` :!label _label_2)
          (:`Update`
            (`SceneComponent.K2_SetRelativeRotation` (`self.StaticMeshDoor`) (`KismetMathLibrary.MakeRotator` 0.0 0.0 _doorrotationamount) false false)))
        (else
          (goto _label_2 :!via `PlayFromStart`))))))

(fn `UserConstructionScript`)