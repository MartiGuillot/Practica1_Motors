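; Coin pickup actor that the third-person character collects for a coin count.
; Tick spins the mesh at RotatorSpeed, scaled by delta time.
; On sphere overlap it spawns an explosion emitter, then, if the other actor is a ThirdPersonCharacter, calls AddCoin, prints the count for debugging and destroys itself.
; An unfinished sine-based hover is left disconnected.
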(event `self.ReceiveTick`
  (params (DeltaSeconds :type "Float (single-precision)"))
  ;[1 1 1] Esto hace que la mesh rote y de un efecto guay
  (`SceneComponent.K2_AddRelativeRotation` (`self.StaticMesh`) (* (`KismetMathLibrary.MakeRotator` 0.0 0.0 (`self.rotatorSpeed`)) DeltaSeconds) false false))

(event `self.SphereCollider.OnComponentBeginOverlap`
  (params (OverlappedComponent :type "PrimitiveComponent Object Reference") (OtherActor :type "Actor Object Reference") (OtherComp :type "PrimitiveComponent Object Reference") (OtherBodyIndex :type Integer) (bFromSweep :type Boolean) (SweepResult :type "HitResult Structure (by ref)"))
  ;[1 1 1] CoinLife (ara falta un contador al hud quan el tinguem)
  (`GameplayStatics.SpawnEmitterAtLocation` "/Game/StarterContent/Particles/P_Explosion.P_Explosion" (.location (`self.GetTransform`)) (.rotation (`self.GetTransform`)) (.scale (`self.GetTransform`)))
  (bind _asthird_person_character (cast `/Game/ThirdPersonBP/Blueprints/ThirdPersonCharacter` OtherActor))
  (`/Game/ThirdPersonBP/Blueprints/ThirdPersonCharacter.AddCoin` _asthird_person_character)
  (`KismetSystemLibrary.PrintString` (`KismetStringLibrary.Conv_IntToString` (`/Game/ThirdPersonBP/Blueprints/ThirdPersonCharacter.numberOfCoins` _asthird_person_character)))
  (`self.K2_DestroyActor`))

(fn `UserConstructionScript`)