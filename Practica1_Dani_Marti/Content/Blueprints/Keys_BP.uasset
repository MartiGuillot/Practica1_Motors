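; Key pickup actor that spins its mesh every tick and is collected when anything overlaps its capsule collider.
; On overlap it hides itself, disables collision, plays a bell sound and sets its own HasCollectedKey flag, without checking the overlapping actor.
; Disconnected leftover nodes for an explosion effect, adding to the ThirdPersonCharacter key count, debug prints and a sine hover never run.
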(event `self.ReceiveTick`
  (params (DeltaSeconds :type "Float (single-precision)"))
  ;[1 1 1] Esto hace que la mesh rote y de un efecto guay
  (`SceneComponent.K2_AddRelativeRotation` (`self.StaticMesh`) (* (`KismetMathLibrary.MakeRotator` 0.0 0.0 (`self.rotatorSpeed`)) DeltaSeconds) false false))

(event `self.CapsuleCollider.OnComponentBeginOverlap`
  (params (OverlappedComponent :type "PrimitiveComponent Object Reference") (OtherActor :type "Actor Object Reference") (OtherComp :type "PrimitiveComponent Object Reference") (OtherBodyIndex :type Integer) (bFromSweep :type Boolean) (SweepResult :type "HitResult Structure (by ref)"))
  ;[1 1 1] CoinLife (ara falta un contador al hud quan el tinguem)
  (`self.SetActorHiddenInGame` true)
  (`self.SetActorEnableCollision` false)
  (`GameplayStatics.PlaySoundAtLocation` "/Game/Sound/bellBeep.bellBeep" (`self.K2_GetActorLocation`) (struct) 1.0 1.0 0.0 null null null)
  (set `self.hasCollectedKey` true))

(fn `UserConstructionScript`)