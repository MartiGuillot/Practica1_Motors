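; Confusion actor that puts a referenced character into a confused state for a limited time.
; Any overlap with its collision box sets IsConfused on the referenced character, without checking which actor overlapped.
; Tick accumulates time while that flag is set, then clears it and resets the timer once MaxConfusion is exceeded.
; Re-overlapping during confusion does not restart the timer.
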(event `self.CollisionBox.OnComponentBeginOverlap`
  (params (OverlappedComponent :type "PrimitiveComponent Object Reference") (OtherActor :type "Actor Object Reference") (OtherComp :type "PrimitiveComponent Object Reference") (OtherBodyIndex :type Integer) (bFromSweep :type Boolean) (SweepResult :type "HitResult Structure (by ref)"))
  (set `/Game/FirstPersonBP/Blueprints/FirstPersonCharacter.isConfused` true (`self.characterReference`)))

(event `self.ReceiveTick`
  (params (DeltaSeconds :type "Float (single-precision)"))
  (if (`/Game/FirstPersonBP/Blueprints/FirstPersonCharacter.isConfused` (`self.characterReference`))
    (bind _output_get (set `self.timeConfused` (+ DeltaSeconds (`self.timeConfused`))))
    (if (> _output_get (`self.maxConfusion`))
      (set `/Game/FirstPersonBP/Blueprints/FirstPersonCharacter.isConfused` false (`self.characterReference`))
      (set `self.timeConfused` 0.0))))

(fn `UserConstructionScript`)