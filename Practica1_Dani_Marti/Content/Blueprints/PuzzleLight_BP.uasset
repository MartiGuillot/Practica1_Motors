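; Puzzle light actor that toggles itself and its left and right neighbor lights, in a Lights Out-style puzzle.
; Any overlap on its Collider flips all three and plays a switch sound, with no cascade beyond those neighbors.
; ActivateLight flips IsLightOn, then swaps point light intensity and cube material.
; ActivateLightForSaveGame applies a given state's visuals without updating IsLightOn.
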(event `self.Collider.OnComponentBeginOverlap`
  (params (OverlappedComponent :type "PrimitiveComponent Object Reference") (OtherActor :type "Actor Object Reference") (OtherComp :type "PrimitiveComponent Object Reference") (OtherBodyIndex :type Integer) (bFromSweep :type Boolean) (SweepResult :type "HitResult Structure (by ref)"))
  (`self.ActivateLight` (`self.LeftLight`))
  (`self.ActivateLight` (`self.RightLight`))
  (`self.ActivateLight`)
  (`GameplayStatics.PlaySoundAtLocation` "/Game/Sound/lightSwitch.lightSwitch" (`self.K2_GetActorLocation`) (struct) 1.0 1.0 0.0 null null null))

(fn `ActivateLight`
  (bind _output_get (set `self.isLightOn` (not (`self.isLightOn`))))
  (if _output_get
    (`LightComponent.SetIntensity` (`self.PointLight`) 10000.0)
    (`PrimitiveComponent.SetMaterial` (`self.Cube`) 0 (`self.materialOn`))
    (else
      (`LightComponent.SetIntensity` (`self.PointLight`) 0.0)
      (`PrimitiveComponent.SetMaterial` (`self.Cube`) 0 (`self.materialOff`)))))

(fn `ActivateLightForSaveGame`
  (params (isLightActivated :type Boolean))
  (if isLightActivated
    (`LightComponent.SetIntensity` (`self.PointLight`) 10000.0)
    (`PrimitiveComponent.SetMaterial` (`self.Cube`) 0 (`self.materialOn`))
    (else
      (`LightComponent.SetIntensity` (`self.PointLight`) 0.0)
      (`PrimitiveComponent.SetMaterial` (`self.Cube`) 0 (`self.materialOff`)))))

(fn `UserConstructionScript`)